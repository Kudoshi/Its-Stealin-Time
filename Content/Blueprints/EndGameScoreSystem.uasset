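; End-of-heist scoring Blueprint that decides success or failure, calculates the player's networth and shows the results screen.
; EndGame combines stolen item and mission values with multipliers for missions completed, time left, alert level and ending the heist; incomplete missions force a loss.
; It freezes time, switches to UI input and fills W_EndGame.
; Per-level bests persist in a LevelBestScore save game, indexed by the GameInstance's loaded level.
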(fn `Calculate Time Taken`
  (params (Minutes :type Integer) (Seconds :type Integer)))

(fn `EndGame`
  (params (EndHeist :type Boolean) (LoseGame :type Boolean))
  (locals (BPPlayer :type "/Game/FirstPerson/Blueprints/BP_Player Object Reference") (AlertMeterSystem :type "/Game/Blueprints/AlertMeterSystem Object Reference") (PlayerPickup :type "/Game/FirstPerson/Blueprints/BP_PlayerPickup Object Reference") (Ov_ItemStolen :type Integer :default 0) (`Ov_Time Left` :type String) (Sum_AlertLevelLabel :type "Float (double-precision)" :default 0.0) (Sum_MissionAccomplished :type Integer :default 0) (Sum_MissionValue :type Integer) (Sum_StolenItemValue :type Integer) (Sum_TimeRemaining :type "Float (double-precision)") (Sum_EndHeist :type Boolean) (Sum_AlertLevelMultiplier :type "Float (double-precision)") (Temp_TotalValue :type "Float (double-precision)") (TotalNetworth :type "Float (double-precision)") (PlayerLoseGame :type Boolean) (Temp_EndHeistMultipler :type "Float (double-precision)") (Temp_BestNetworth :type String) (Temp_Networth :type String))
  (bind _returnvalue (`GameplayStatics.GetPlayerController` 0))
  (bind _bpplayer (`local.BPPlayer`))
  (bind _bpplayer_2 (`local.BPPlayer`))
  (set `local.PlayerLoseGame` LoseGame)
  (set `local.Sum_EndHeist` EndHeist)
  (`|ExecutionSequence`
    (:`then_0`
      (bind _asbp_player (cast `/Game/FirstPerson/Blueprints/BP_Player` (`GameplayStatics.GetPlayerCharacter` 0)))
      (bind _output_get (set `local.BPPlayer` _asbp_player))
      (set `local.PlayerPickup` (`/Game/FirstPerson/Blueprints/BP_Player.BP_PlayerPickup` _output_get))
      (bind _asthief_game_mode (cast `/Game/Blueprints/ThiefGameMode` (`GameplayStatics.GetGameMode`)))
      (set `local.AlertMeterSystem` (`/Game/Blueprints/ThiefGameMode.AlertMeterSystem` _asthief_game_mode)))
    (:`then_1`
      (set `local.Ov_ItemStolen` (`KismetArrayLibrary.Array_Length` (`/Game/FirstPerson/Blueprints/BP_PlayerPickup.AllStolenItemArray` (`local.PlayerPickup`))))
      (set `local.Ov_Time Left` (`KismetStringLibrary.Concat_StrStr` (`KismetStringLibrary.Concat_StrStr` (`KismetStringLibrary.Conv_IntToString` (`Timer.Minutes` _bpplayer_2)) " m ") (`KismetStringLibrary.Concat_StrStr` (`KismetStringLibrary.Conv_IntToString` (`Timer.Seconds` _bpplayer_2)) " s"))))
    (:`then_2`
      (set `local.Sum_AlertLevelLabel` (* (`/Game/Blueprints/AlertMeterSystem.AlertPoints` (`local.AlertMeterSystem`)) 100.0))
      (bind _returnvalue_2 (`MissionManager.GetCurrentLevelMission` (subsystem `MissionManager`)))
      (for _array_element _returnvalue_2
        (bind (_missiondescription _missionobjective _missionvalue _completed) (break `Mission` _array_element))
        (if _completed
          (set `local.Sum_MissionAccomplished` (+ (`local.Sum_MissionAccomplished`) 1))
          (set `local.Sum_MissionValue` (+ (`local.Sum_MissionValue`) _missionvalue))))
      (for _array_element_2 (`/Game/FirstPerson/Blueprints/BP_PlayerPickup.AllStolenItemArray` (`local.PlayerPickup`))
        (set `local.Sum_StolenItemValue` (+ (`local.Sum_StolenItemValue`) (`.itemValue` (break `GameItem` _array_element_2)))))
      (set `local.Sum_TimeRemaining` (/ (/ (+ (`Timer.Seconds` _bpplayer) (* (`Timer.Minutes` _bpplayer) 60)) (`self.MaxGameTime`)) 2.0))
      (set `local.Sum_AlertLevelMultiplier` (/ (- 100.0 (`/Game/Blueprints/AlertMeterSystem.AlertPoints` (`local.AlertMeterSystem`))) 100.0)))
    (:`then_3`
      (bind _returnvalue_3 (`MissionManager.GetCurrentLevelMission` (subsystem `MissionManager`)))
      (if (not (== (`KismetArrayLibrary.Array_Length` _returnvalue_3) (`local.Sum_MissionAccomplished`)))
        (set `local.PlayerLoseGame` true)))
    (:`then_4`
      (if (`local.PlayerLoseGame`)
        (set `local.Sum_AlertLevelLabel` 0.0)
        (set `local.Sum_MissionAccomplished` 0)
        (set `local.Sum_TimeRemaining` 0.0)
        (set `local.Sum_AlertLevelMultiplier` 0.0)
        (bind _output_get_2 (set `local.TotalNetworth` 0.0))
        (set `local.Temp_EndHeistMultipler` _output_get_2)
        (else
          (set `local.Temp_TotalValue` (+ (`local.Sum_StolenItemValue`) (`local.Sum_MissionValue`)))
          (set `local.TotalNetworth` (+ (* (`local.Temp_TotalValue`) (/ (`KismetMathLibrary.Conv_IntToDouble` (`local.Sum_MissionAccomplished`)) 10.0)) (+ (* (`local.Temp_TotalValue`) (`local.Sum_AlertLevelMultiplier`)) (+ (`local.Temp_TotalValue`) (* (`local.Temp_TotalValue`) (`local.Sum_TimeRemaining`))))))
          (if (`local.Sum_EndHeist`)
            (set `local.TotalNetworth` (+ (`local.TotalNetworth`) (* (`local.Temp_TotalValue`) (`self.EndHeistMultiplier`))))
            (if (`local.Sum_EndHeist`)
              (set `local.Temp_EndHeistMultipler` (`self.EndHeistMultiplier`))
              (else
                (set `local.Temp_EndHeistMultipler` 0.0)))))))
    (:`then_5`
      (`GameplayStatics.SetGlobalTimeDilation` 0.0)
      (`Actor.DisableInput` (`local.BPPlayer`) null)
      (`WidgetBlueprintLibrary.SetInputMode_UIOnlyEx` _returnvalue null "DoNotLock" true)
      (set `PlayerController.bShowMouseCursor` true _returnvalue)
      (`|ExecutionSequence`
        (:`then_0`
          (bind _bestnetworth (`self.GetPlayerBestNetworth`))
          (if (> (`local.TotalNetworth`) _bestnetworth)
            (set `local.Temp_BestNetworth` "- NEW BEST - ")
            (`self.Save Player Best Networth` (`local.TotalNetworth`))
            (else
              (set `local.Temp_BestNetworth` (`KismetStringLibrary.Concat_StrStr` "$ " (`KismetTextLibrary.Conv_TextToString` (`KismetTextLibrary.Conv_DoubleToText` _bestnetworth "HalfToEven" false true 1 324 2 2)))))))
        (:`then_1`
          (if (or (== (`local.TotalNetworth`) 0.0) (== (`local.PlayerLoseGame`) true))
            (set `local.Temp_Networth` "HEIST FAIL")
            (else
              (set `local.Temp_Networth` (`KismetStringLibrary.Concat_StrStr` "$ " (`KismetTextLibrary.Conv_TextToString` (`KismetTextLibrary.Conv_DoubleToText` (`local.TotalNetworth`) "HalfToEven" false true 1 324 2 2)))))))
        (:`then_2`
          (bind _returnvalue_4 (`|CreateWidget` "/Game/UI/W_EndGame.W_EndGame_C"))
          (`UserWidget.AddToViewport` _returnvalue_4 0)
          (`/Game/UI/W_EndGame.Load Values` _returnvalue_4 (`local.Temp_BestNetworth`) (`KismetStringLibrary.Conv_IntToString` (`local.Ov_ItemStolen`)) (`local.Ov_Time Left`) (`local.Temp_Networth`) (`KismetStringLibrary.Concat_StrStr` "x " (`KismetTextLibrary.Conv_TextToString` (`KismetTextLibrary.Conv_DoubleToText` (`local.Sum_AlertLevelMultiplier`) "HalfToEven" false true 1 324 2 2))) (`KismetStringLibrary.Concat_StrStr` "x " (`KismetTextLibrary.Conv_TextToString` (`KismetTextLibrary.Conv_DoubleToText` (/ (`KismetMathLibrary.Conv_IntToDouble` (`local.Sum_MissionAccomplished`)) 10.0) "HalfToEven" false true 1 324 2 2))) (`KismetStringLibrary.Concat_StrStr` "$ " (`KismetTextLibrary.Conv_TextToString` (`KismetTextLibrary.Conv_DoubleToText` (`KismetMathLibrary.Conv_IntToDouble` (`local.Sum_MissionValue`)) "HalfToEven" false true 1 324 2 2))) (`KismetStringLibrary.Concat_StrStr` "$ " (`KismetTextLibrary.Conv_TextToString` (`KismetTextLibrary.Conv_DoubleToText` (`KismetMathLibrary.Conv_IntToDouble` (`local.Sum_StolenItemValue`)) "HalfToEven" false true 1 324 2 2))) (`KismetStringLibrary.Concat_StrStr` "x " (`KismetTextLibrary.Conv_TextToString` (`KismetTextLibrary.Conv_DoubleToText` (`local.Sum_TimeRemaining`) "HalfToEven" false true 1 324 2 2))) (`KismetStringLibrary.Concat_StrStr` "x " (`KismetTextLibrary.Conv_TextToString` (`KismetTextLibrary.Conv_DoubleToText` (`local.Temp_EndHeistMultipler`) "HalfToEven" false true 1 324 2 2))) (`KismetStringLibrary.Concat_StrStr` (`KismetTextLibrary.Conv_TextToString` (`KismetTextLibrary.Conv_DoubleToText` (`/Game/Blueprints/AlertMeterSystem.AlertPoints` (`local.AlertMeterSystem`)) "HalfToEven" false true 1 324 0 0)) "%")))))))

(fn `GetPlayerBestNetworth`
  (returns (BestNetworth :type "Float (double-precision)"))
  (bind _returnvalue (`GameplayStatics.DoesSaveGameExist` (`self.SaveGameSlot`)))
  (if _returnvalue
    (bind _returnvalue_2 (`GameplayStatics.LoadGameFromSlot` (`self.SaveGameSlot`)))
    (bind _aslevel_best_score (cast `/Game/Blueprints/LevelBestScore` _returnvalue_2))
    (bind _asthief_game_instance (cast `/Game/Blueprints/ThiefGameInstance` (`GameplayStatics.GetGameInstance`)))
    (return (`|GetArrayItem` (`/Game/Blueprints/LevelBestScore.BestNetworth` _aslevel_best_score) (- (`/Game/Blueprints/ThiefGameInstance.LoadedLevel` _asthief_game_instance) 1)))
    (else
      (return 0.0))))

(fn `Save Player Best Networth`
  (params (NewBestNetworth :type "Float (double-precision)"))
  (locals (BestNetworth :type "Float (double-precision)") (LevelArrIndex :type Integer) (SaveBestScore :type "/Game/Blueprints/LevelBestScore Object Reference"))
  (set `local.BestNetworth` NewBestNetworth)
  (`|ExecutionSequence`
    (:`then_0`
      (bind _asthief_game_instance (cast `/Game/Blueprints/ThiefGameInstance` (`GameplayStatics.GetGameInstance`)))
      (set `local.LevelArrIndex` (- (`/Game/Blueprints/ThiefGameInstance.LoadedLevel` _asthief_game_instance) 1)))
    (:`then_1`
      (bind _returnvalue (`GameplayStatics.DoesSaveGameExist` (`self.SaveGameSlot`)))
      (if _returnvalue
        (bind _returnvalue_2 (`GameplayStatics.LoadGameFromSlot` (`self.SaveGameSlot`)))
        (bind _aslevel_best_score (cast `/Game/Blueprints/LevelBestScore` _returnvalue_2))
        (set `local.SaveBestScore` _aslevel_best_score)
        (`KismetArrayLibrary.Array_Set` (`/Game/Blueprints/LevelBestScore.BestNetworth` _aslevel_best_score) (`local.LevelArrIndex`) (`local.BestNetworth`))
        (else
          (bind _returnvalue_3 (`GameplayStatics.CreateSaveGameObject` "/Game/Blueprints/LevelBestScore.LevelBestScore_C"))
          (set `local.SaveBestScore` _returnvalue_3)
          (`KismetArrayLibrary.Array_Set` (`/Game/Blueprints/LevelBestScore.BestNetworth` _returnvalue_3) (`local.LevelArrIndex`) (`local.BestNetworth`))))
      (`GameplayStatics.SaveGameToSlot` (`local.SaveBestScore`) (`self.SaveGameSlot`)))))