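; ThiefGameInstance is the game instance that switches the game between the main menu and numbered levels.
; LoadLevel clears the current mission through the MissionManager, then opens the main menu for level 0 or the shared main map for any other number.
; For gameplay levels it initializes the mission named after the level number right after the open-level call, so all levels share one map.
; It records the loaded level number, and Init is empty.
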(event `self.ReceiveInit`)

(fn `LoadLevel`
  (params (Level :type Integer))
  (locals (`Level ` :type Integer))
  (bind _returnvalue (subsystem `MissionManager`))
  (set `local.Level ` Level)
  (`MissionManager.DeinitializeLevelMissionInStage` _returnvalue)
  (if (== (`local.Level `) 0)
    (`GameplayStatics.OpenLevelBySoftObjectPtr` "/Game/Map/MainMenu_Level.MainMenu_Level")
    (else
      (`GameplayStatics.OpenLevelBySoftObjectPtr` "/Game/Map/MainLevelMap.MainLevelMap")
      (`MissionManager.InitializeLevelMissionInStage` _returnvalue (`KismetStringLibrary.Conv_StringToName` (`KismetStringLibrary.Conv_IntToString` (`local.Level `))))))
  (set `self.LoadedLevel` (`local.Level `)))