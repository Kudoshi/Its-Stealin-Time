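; Alert meter system that tracks the player's alert level and triggers game over when it maxes out.
; AddAlertPoints raises the level, optionally lifting a permanent floor, and displays the HUD manager's game-over screen at the cap.
; A looping timer decays the level toward that floor and updates the HUD meter.
; Each decay tick also drives a heartbeat sound that plays at high alert, rising in pitch as the meter fills.
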(event `self.ReceiveBeginPlay`
  (`KismetSystemLibrary.DelayUntilNextTick`)
  (bind _ashudlevel_manager (cast `/Game/Blueprints/HUDLevel_Manager` (`PlayerController.GetHUD` (`GameplayStatics.GetPlayerController` 0)))
    (:`then`
      (set `self.Game UI` (`/Game/Blueprints/HUDLevel_Manager.GameUI` _ashudlevel_manager))
      (bind _returnvalue (`GameplayStatics.CreateSound2D` "/Game/Sounds/SoundEffects/SFX_Heart_Beat_Cleaned.SFX_Heart_Beat_Cleaned" 1.0 1.0 0.0 null false false))
      (set `self.AlertAudio` _returnvalue)
      (bind _returnvalue_2 (`KismetSystemLibrary.K2_SetTimer` null "AlertDecay" 0.1 true))
      (set `self.AlertDecayTimer` _returnvalue_2))
    (:`CastFailed`
      (`KismetSystemLibrary.PrintString` "HUDLevel_Manager Not Found"))))

(fn `Add Alert Points`
  (params (AlertPoints :type "Float (double-precision)") (PermanentPoints :type Boolean))
  (locals (AlertPointInput :type "Float (double-precision)"))
  (bind _game_ui (`self.Game UI`))
  (bind _returnvalue (+ (`self.AlertPoints`) (`local.AlertPointInput`)))
  (set `local.AlertPointInput` AlertPoints)
  (if PermanentPoints
    (set `self.AlertPermanentPoints` (+ AlertPoints (`self.AlertPermanentPoints`))))
  (if (>= _returnvalue 100.0)
    (bind _output_get (set `self.AlertPoints` 100.0))
    (`/Game/UI/GameUI.Update Alert Meter` _game_ui _output_get)
    (set `self.GameOver` true)
    (bind _ashudlevel_manager (cast `/Game/Blueprints/HUDLevel_Manager` (`PlayerController.GetHUD` (`GameplayStatics.GetPlayerController` 0))))
    (`/Game/FirstPerson/Blueprints/Game_Over/GameOver.DisplayGameOver` (`/Game/Blueprints/HUDLevel_Manager.GameOverUI` _ashudlevel_manager))
    (else
      (bind _output_get_2 (set `self.AlertPoints` _returnvalue))
      (`/Game/UI/GameUI.Update Alert Meter` _game_ui _output_get_2))))

(fn `AlertDecay`
  (locals (PointAfterDecrease :type "Float (double-precision)"))
  (if (not (`self.GameOver`))
    (set `local.PointAfterDecrease` (- (`self.AlertPoints`) (`self.AlertDecreasePoint`)))
    (if (< (`local.PointAfterDecrease`) (`self.AlertPermanentPoints`))
      (set `self.AlertPoints` (`self.AlertPermanentPoints`))
      (else
        (set `self.AlertPoints` (`local.PointAfterDecrease`))))
    (bind _game_ui (`self.Game UI`)
      (:`then`
        (`/Game/UI/GameUI.Update Alert Meter` _game_ui (`self.AlertPoints`))
        (`self.PlayAlertAudio`))
      (:`else`))))

(fn `PlayAlertAudio`
  (bind _alertaudio (`self.AlertAudio`))
  (if (>= (`self.AlertPoints`) 75.0)
    (`AudioComponent.SetPitchMultiplier` _alertaudio (`KismetMathLibrary.MapRangeClamped` (`self.AlertPoints`) 75.0 100.0 1.0 3.0))
    (if (not (`AudioComponent.IsPlaying` _alertaudio))
      (`AudioComponent.Play` _alertaudio 0.0))
    (elif (`AudioComponent.IsPlaying` _alertaudio)
      (`AudioComponent.Stop` _alertaudio))))